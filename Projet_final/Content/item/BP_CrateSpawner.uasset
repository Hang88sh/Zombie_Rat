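; BP_CrateSpawner is a spawner that periodically creates BP_WoodenCrate actors up to a small fixed limit.
; BeginPlay starts a looping timer that calls SpawnCrate, which checks and increments CrateCount.
; Each crate gets a random X/Y position bounded by SpawnRadius at zero height, without adding the spawner's own location.
; CrateCount never decreases, so the limit caps total spawns rather than live crates.
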(event Custom|SpawnCrate
  (if (< (Variables|Default|GetCrateCount) 5)
    (Game|SpawnActorfromClass "/Game/item/BP_WoodenCrate.BP_WoodenCrate_C" (Math|Conversions|ToTransform(Vector) (Math|Vector|MakeVector (Math|Random|RandomFloatinRange (stale _result) (Variables|Default|GetSpawnRadius%20)) (Math|Random|RandomFloatinRange (stale _result) (Variables|Default|GetSpawnRadius%20)) 0.0)) "Undefined" "MultiplyWithRoot" 0 0)
    (Variables|Default|SetCrateCount (+ (Variables|Default|GetCrateCount) 1))))

(event EventBeginPlay
  (Utilities|Time|SetTimerbyEvent (delegate Custom|SpawnCrate) 5.0 true))

(fn ConstructionScript)